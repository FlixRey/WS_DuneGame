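; Race manager Blueprint that runs the race start: setup, HUD countdown, then launch of the AI cars.
; On BeginPlay it binds checkpoint events on the AI cars, caches the player car and HUD, and seeds per-lap position entries from RaceDatas.
; After the countdown delay, StartRace sends the start message to AI cars only.
; The checkpoint handler is empty and the player car's start call is unconnected.
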(event `PassCheckpoint`
  (params (Car :type "/Game/VehicleTemplate/Blueprints/IA/BP_IACar Object Reference")))

(event `self.ReceiveBeginPlay`
  (bind (_racedatas_countdownduration _racedatas_countdownendmessage) (break `/Game/VehicleTemplate/Blueprints/IA/ST_RaceData` (`self.RaceDatas`)))
  (`|ExecutionSequence`
    (:`then_0`
      (for _array_element (`self.CarsIA`)
        (add `/Game/VehicleTemplate/Blueprints/IA/BP_IACar.OnPassedCheckPoint` _array_element (delegate `PassCheckpoint`))))
    (:`then_1`
      (`KismetSystemLibrary.Delay` 0.1)
      (`self.InitRace`)
      (`/Game/VehicleTemplate/Blueprints/IA/BPW_MainHUD.CountDown` (`self.HUD`) _racedatas_countdownduration _racedatas_countdownendmessage)
      (`KismetSystemLibrary.Delay` (`KismetMathLibrary.Conv_IntToDouble` _racedatas_countdownduration))
      (`self.StartRace`))))

(fn `InitRace`
  (bind (_racedatas_countdownduration _racedatas_countdownendmessage _racedatas_lapnumber) (break `/Game/VehicleTemplate/Blueprints/IA/ST_RaceData` (`self.RaceDatas`)))
  (bind _asbp_car_pawn (cast `/Game/VehicleTemplate/Blueprints/IA/BP_CarPawn` (`GameplayStatics.GetPlayerPawn` 0)))
  (set `self.PlayerCar` _asbp_car_pawn)
  (set `self.HUD` (`/Game/VehicleTemplate/Blueprints/IA/BP_CarPawn.HUD` _asbp_car_pawn))
  (for _ (range (+ _racedatas_lapnumber 1))
    (`KismetArrayLibrary.Array_Add` (`self.LapTurnPositions`) 1)))

(fn `StartRace`
  (for _array_element (`self.CarsIA`)
    (message `/Game/VehicleTemplate/Blueprints/IA/BPI_CarInRace.StartRace` _array_element)))

(fn `UserConstructionScript`)