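; Green AI ship Blueprint that travels along the spline of the Pathfinding_vert actor.
; On BeginPlay it finds that actor by class and starts the Speed timeline, with play rate set to the inverse of TimeToComplite.
; Each update maps the timeline track onto spline length and sets the ship's transform from world-space location and local-space rotation at that distance.
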(event `self.ReceiveBeginPlay`
  (bind _returnvalue (`GameplayStatics.GetActorOfClass` "/Game/VaisseauxIA/Veceau_vert/pathfinding_vert.pathfinding_vert_C"))
  (set `self.splin vert` _returnvalue)
  (`self.move`))

(event `move`
  (bind _spline (`/Game/VaisseauxIA/Veceau_vert/pathfinding_vert.Spline` (`self.splin vert`)))
  (`TimelineComponent.SetPlayRate` (`self.speed`) (/ 1.0 (`self.time to complite`)))
  (bind (_direction _move_track) (`Timeline|speed`)
    (:`Update`
      (bind _returnvalue (`KismetMathLibrary.Lerp` 0.0 (`SplineComponent.GetSplineLength` (`/Game/VaisseauxIA/Veceau_vert/pathfinding_vert.Spline` (`self.splin vert`))) _move_track))
      (`self.K2_SetActorTransform` (`KismetMathLibrary.MakeTransform` (`SplineComponent.GetLocationAtDistanceAlongSpline` _spline _returnvalue "World") (`SplineComponent.GetRotationAtDistanceAlongSpline` _spline _returnvalue "Local"))))))

(fn `UserConstructionScript`)