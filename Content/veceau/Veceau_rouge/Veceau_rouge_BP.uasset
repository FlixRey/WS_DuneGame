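; Red "veceau" actor Blueprint that travels along the spline of the Pathfinding_rouge actor.
; On BeginPlay it finds that actor, stores it and starts the Speed timeline, with play rate set to the inverse of TimeToComplite.
; Each update maps MoveTrack to a distance along the spline and sets the actor's transform, taking location in world space but rotation in local space.
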(event `self.ReceiveBeginPlay`
  (bind _returnvalue (`GameplayStatics.GetActorOfClass` "/Game/veceau/Veceau_rouge/pathfinding_rouge.pathfinding_rouge_C"))
  (set `self.splin rouge` _returnvalue)
  (`self.move`))

(event `move`
  (bind _spline (`/Game/veceau/Veceau_rouge/pathfinding_rouge.Spline` (`self.splin rouge`)))
  (`TimelineComponent.SetPlayRate` (`self.speed`) (/ 1.0 (`self.time to complite`)))
  (bind (_direction _move_track) (`Timeline|speed`)
    (:`Update`
      (bind _returnvalue (`KismetMathLibrary.Lerp` 0.0 (`SplineComponent.GetSplineLength` (`/Game/veceau/Veceau_rouge/pathfinding_rouge.Spline` (`self.splin rouge`))) _move_track))
      (`self.K2_SetActorTransform` (`KismetMathLibrary.MakeTransform` (`SplineComponent.GetLocationAtDistanceAlongSpline` _spline _returnvalue "World") (`SplineComponent.GetRotationAtDistanceAlongSpline` _spline _returnvalue "Local"))))))

(fn `UserConstructionScript`)