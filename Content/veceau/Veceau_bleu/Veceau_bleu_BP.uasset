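; Veceau_bleu_BP is an actor that travels along the blue pathfinding spline from start to end.
; On BeginPlay it finds the Pathfinding_bleu actor in the level and starts the Move event.
; A Speed timeline, with play rate set from TimeToComplite, drives a lerp over the spline length.
; Each update sets the actor's location in world space and its rotation from the spline's local space.
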(event `self.ReceiveBeginPlay`
  (bind _returnvalue (`GameplayStatics.GetActorOfClass` "/Game/veceau/Veceau_bleu/pathfinding_bleu.pathfinding_bleu_C"))
  (set `self.splin bleu` _returnvalue)
  (`self.move`))

(event `move`
  (bind _spline (`/Game/veceau/Veceau_bleu/pathfinding_bleu.Spline` (`self.splin bleu`)))
  (`TimelineComponent.SetPlayRate` (`self.speed`) (/ 1.0 (`self.time to complite`)))
  (bind (_direction _move_track) (`Timeline|speed`)
    (:`Update`
      (bind _returnvalue (`KismetMathLibrary.Lerp` 0.0 (`SplineComponent.GetSplineLength` (`/Game/veceau/Veceau_bleu/pathfinding_bleu.Spline` (`self.splin bleu`))) _move_track))
      (`self.K2_SetActorTransform` (`KismetMathLibrary.MakeTransform` (`SplineComponent.GetLocationAtDistanceAlongSpline` _spline _returnvalue "World") (`SplineComponent.GetRotationAtDistanceAlongSpline` _spline _returnvalue "Local"))))))

(fn `UserConstructionScript`)