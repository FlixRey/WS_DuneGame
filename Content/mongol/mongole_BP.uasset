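; Mongol actor Blueprint that travels along a spline path once play begins.
; On BeginPlay it finds a Pathfinding_mongole actor in the level and starts the Speed timeline, with play rate set to the inverse of TimeToComplite.
; Each update maps the timeline track to a distance along the spline, setting the actor's location from world space and its rotation from local space.
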(event `self.ReceiveBeginPlay`
  (bind _returnvalue (`GameplayStatics.GetActorOfClass` "/Game/mongol/pathfinding_mongole.pathfinding_mongole_C"))
  (set `self.spline mongole` _returnvalue)
  (`self.move`))

(event `move`
  (bind _spline (`/Game/mongol/pathfinding_mongole.Spline` (`self.spline mongole`)))
  (`TimelineComponent.SetPlayRate` (`self.speed`) (/ 1.0 (`self.time to complite`)))
  (bind (_direction _move_track) (`Timeline|speed`)
    (:`Update`
      (bind _returnvalue (`KismetMathLibrary.Lerp` 0.0 (`SplineComponent.GetSplineLength` (`/Game/mongol/pathfinding_mongole.Spline` (`self.spline mongole`))) _move_track))
      (`self.K2_SetActorTransform` (`KismetMathLibrary.MakeTransform` (`SplineComponent.GetLocationAtDistanceAlongSpline` _spline _returnvalue "World") (`SplineComponent.GetRotationAtDistanceAlongSpline` _spline _returnvalue "Local"))))))

(fn `UserConstructionScript`)