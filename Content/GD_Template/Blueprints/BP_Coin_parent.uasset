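; Parent coin pickup Blueprint that the player's vehicle collects by driving into it.
; When the player pawn overlaps the Sphere, a DoOnce gate casts it to BP_CustomPlayerVehicule, increments its Coins counter and destroys the coin.
; Unconnected leftover nodes would raise the vehicle's engine torque on pickup and loop over its wheels, but they never run.
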(event `self.Sphere.OnComponentBeginOverlap`
  (params (OverlappedComponent :type "PrimitiveComponent Object Reference") (OtherActor :type "Actor Object Reference") (OtherComp :type "PrimitiveComponent Object Reference") (OtherBodyIndex :type Integer) (bFromSweep :type Boolean) (SweepResult :type "HitResult Structure (by ref)"))
  (bind _returnvalue (`GameplayStatics.GetPlayerPawn` 0))
  (if (== _returnvalue OtherActor)
    (`/Engine/EditorBlueprintResources/StandardMacros.DoOnce` false
      (:`Completed`
        (bind _asbp_custom_player_vehicule (cast `/Game/GD_Template/Blueprints/BP_CustomPlayerVehicule` _returnvalue))
        (`/Engine/EditorBlueprintResources/StandardMacros.IncrementInt` (`/Game/GD_Template/Blueprints/BP_CustomPlayerVehicule.Coins` _asbp_custom_player_vehicule)
          (:`  `
            (`self.K2_DestroyActor`)))))))

(fn `UserConstructionScript`)